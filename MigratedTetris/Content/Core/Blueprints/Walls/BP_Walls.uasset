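; BP_Walls is a wall Blueprint that plays a fade effect on collision.
; Its OnCollision event creates a player for the LS_CollisionFade level sequence and plays it, creating a new one on each call.
; Older visibility logic, a brief timed show/hide of the Wall component and a StartingVisibility setup in construction, remains disconnected and never runs.
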(event `OnCollision`
  (bind _outactor (`LevelSequencePlayer.CreateLevelSequencePlayer` "/Game/Core/Materials/Color/LS_CollisionFade.LS_CollisionFade"))
  (`MovieSceneSequencePlayer.Play` (`LevelSequenceActor.SequencePlayer` _outactor)))

(fn `UserConstructionScript`)