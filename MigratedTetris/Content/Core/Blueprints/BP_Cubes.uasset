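; BP_Cubes is a cube actor that flashes once when play begins and can destroy a given cube component.
; BeginPlay creates a dynamic material from StoredMaterial and applies it to the Cube.
; The LerpFlashIntensity timeline drives the FlashIntensity parameter up, then reverses once it ends at full alpha to fade it back down.
; DestroyCubes is a separate function that destroys the component passed to it.
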(event `self.ReceiveBeginPlay`
  (bind _returnvalue (`PrimitiveComponent.CreateDynamicMaterialInstance` (`self.Cube`) 0 (`self.StoredMaterial`) "None"))
  (set `self.DMI_Stored_Mat` _returnvalue)
  (`PrimitiveComponent.SetMaterial` (`self.Cube`) 0 (`self.DMI_Stored_Mat`))
  (bind (_direction _alphatrack) (`Timeline|LerpFlashIntensity` :!label _label)
    (:`Update`
      (`MaterialInstanceDynamic.SetScalarParameterValue` (`self.DMI_Stored_Mat`) "FlashIntensity" (`KismetMathLibrary.Lerp` 0.0 75.0 _alphatrack)))
    (:`Finished`
      (if (== _alphatrack 1.0)
        (goto _label :!via `ReverseFromEnd`)))))

(fn `DestroyCubes`
  (params (Cube :type "StaticMeshComponent Object Reference"))
  (`ActorComponent.K2_DestroyComponent` Cube))

(fn `UserConstructionScript`)