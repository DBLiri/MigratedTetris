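; Player-controlled falling piece for 3D Tetris, stepping down on a timer at the game mode's block speed.
; Keys drive timeline-animated moves and pitch/yaw rotations, gated by per-cube line traces.
; Blocked rotations flash red and animate back.
; When blocked below, it passes its cubes to the grid manager (spawns loose cubes in MenuLevel), destroys itself, then requests the next piece or shows game over at spawn height.
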(event `CallTimeline`
  (params (StartLocation :type "Vector Structure") (EndLocation :type "Vector Structure"))
  ;[1 1 1] CallTimeline (MoveDown)
  (bind (_direction _movepeicedown) (`Timeline|TimelineMovePeiceDown` :!via `PlayFromStart`)
    (:`Update`
      (`self.K2_SetActorLocation` (`KismetMathLibrary.VLerp` StartLocation EndLocation _movepeicedown)))))

(event `Key|Up`
  (params (Key :type "Key Structure"))
  (bind _returnvalue (`self.K2_GetActorRotation`))
  ;[1 1 1] Rotation
  ;;[1 1 1] Rotate Pitch
  (:`Pressed`
    (if (not (`self.IsMoving`))
      (set `self.IsMoving` true)
      (`KismetSystemLibrary.PrintString` (`KismetStringLibrary.Conv_RotatorToString` _returnvalue) (`self.PrintDebugMovement`) true (struct :`R` 0.957218 :`G` 1.0 :`A` 1.0) 20.0)
      (set `self.StartingPeiceRotation` _returnvalue)
      (set `self.DetectBoundryDirection` (0.0 0.0 -50.0))
      (set `self.PreviousTimelineValue` 0.0)
      (bind (_direction _yaw) (`Timeline|Timeline_Rotate` :!via `PlayFromStart`)
        (:`Update`
          ;;;[1 1 1] Timeline Body
          (`self.K2_AddActorWorldRotation` (`KismetMathLibrary.MakeRotator` 0.0 (- _yaw (`self.PreviousTimelineValue`))))
          (set `self.PreviousTimelineValue` _yaw)
          ;;;[1 1 1] Comment
          (bind _canmoveoutput (`self.DetectBoundry`))
          (if (not _canmoveoutput)
            (`self.BoundryFlashOn`)))
        (:`Finished`
          (bind _canmoveoutput_2 (`self.DetectBoundryRotate`))
          (if _canmoveoutput_2
            (`KismetSystemLibrary.PrintString` "No Boundry Detected" (`self.PrintDebugRotation`) true (struct :`G` 1.0 :`B` 0.073006 :`A` 1.0) 20.0)
            (set `self.CurrentPeiceRotation` (`self.K2_GetActorRotation`))
            (set `self.IsMoving` false)
            (`self.BoundryFlashoff` :!label _label)
            (else
              (`KismetSystemLibrary.PrintString` "Boundry Detected" (`self.PrintDebugRotation`) true (struct :`R` 1.0 :`G` 0.059606 :`A` 1.0) 20.0)
              ;;;[1 1 1] Animate undo Rotation
              (set `self.PreviousTimelineValue` 0.0)
              (bind (_direction_2 _yaw_2) (`Timeline|Timeline_6` :!via `PlayFromStart`)
                (:`Update`
                  ;;;;[1 1 1] Timeline Body
                  (`self.K2_AddActorWorldRotation` (`KismetMathLibrary.MakeRotator` 0.0 (- (`self.PreviousTimelineValue`) _yaw_2)))
                  (bind _output_get (set `self.PreviousTimelineValue` _yaw_2))
                  (`KismetSystemLibrary.PrintString` (`KismetStringLibrary.Conv_DoubleToString` _output_get) (`self.PrintDebugRotation`) true (struct :`G` 0.66 :`B` 1.0 :`A` 1.0) 20.0))
                (:`Finished`
                  (set `self.CurrentPeiceRotation` (`self.StartingPeiceRotation`))
                  (set `self.IsMoving` false)
                  (goto _label))))))))))

(event `Key|SpaceBar`
  (params (Key :type "Key Structure"))
  ;[1 1 1] Translate Blocks Down (From Input)
  (:`Pressed`
    (if (not (`self.IsMoving`))
      (set `self.IsMoving` true)
      (`self.MovePeiceDown`)
      (set `self.IsMoving` false))))

(event `self.ReceiveTick`
  (params (DeltaSeconds :type "Float (single-precision)"))
  ;[1 1 1] Event Tick
)

(event `Key|W`
  (params (Key :type "Key Structure"))
  (bind _returnvalue (`self.K2_GetActorLocation`))
  ;[1 1 1] Translate Blocks
  ;;[1 1 1] Translate X Front Back
  (:`Pressed`
    (if (not (`self.IsMoving`))
      (set `self.IsMoving` true)
      (set `self.DetectBoundryDirection` (-100.0 0.0 0.0))
      (bind _canmoveoutput (`self.DetectBoundry`))
      (if _canmoveoutput
        (set `self.StartLocation` (`KismetMathLibrary.Vector_SnappedToGrid` _returnvalue (`self.PlayfieldCubeSize`)))
        (set `self.EndLocation` (`KismetMathLibrary.Vector_SnappedToGrid` (`KismetMathLibrary.MakeVector` (- (.x _returnvalue) 100.0) (.y _returnvalue) (.z _returnvalue)) (`self.PlayfieldCubeSize`)))
        (bind (_direction _0_1) (`Timeline|Timeline_0` :!via `PlayFromStart`)
          (:`Update`
            (`self.K2_SetActorLocation` (`KismetMathLibrary.VLerp` (`self.StartLocation`) (`self.EndLocation`) _0_1)))
          (:`Finished`
            (set `self.IsMoving` false)))
        (else
          (set `self.IsMoving` false))))))

(event `self.ReceiveBeginPlay`
  (bind _pausemenuref (`self.PauseMenuRef`))
  ;[1 1 1] Event Begin Play
  (`self.EnableInput` (`GameplayStatics.GetPlayerController` 0))
  (bind _returnvalue (`GameplayStatics.GetActorOfClass` "/Game/Core/Blueprints/BP_Playfeild.BP_Playfeild_C"))
  (bind _output_get (set `self.PlayfeildRef` _returnvalue))
  (bind (_min _max) (`StaticMeshComponent.GetLocalBounds` (`/Game/Core/Blueprints/BP_Playfeild.Cube` _output_get)))
  (set `self.PlayfieldCubeSize` (+ (`KismetMathLibrary.Abs` (.x _min)) (`KismetMathLibrary.Abs` (.x _max))))
  (set `self.PrintDebugMovement` false)
  (set `self.PrintDebugOther` false)
  (`|ExecutionSequence`
    (:`then_0`
      ;[1 1 1] Current Level
      (bind _returnvalue_2 (`GameplayStatics.GetCurrentLevelName` true))
      (set `self.CurrentLevel` _returnvalue_2)
      ;[1 1 1] Starting Matt
      (`self.GetStartingMat`)
      ;[1 1 1] Pause Menu Set Up
      (bind _returnvalue_3 (`|CreateWidget` "/Game/Core/Blueprints/UserInterface/WBP_PauseMenu.WBP_PauseMenu_C"))
      (set `self.PauseMenuRef` _returnvalue_3)
      (`UserWidget.AddToViewport` _pausemenuref 1)
      (`Widget.SetVisibility` _pausemenuref "Hidden")
      ;[1 1 1] Game mode ref
      (bind _astetris_game_mode (cast `/Game/Core/Blueprints/TetrisGameMode` (`GameplayStatics.GetGameMode`)))
      (bind _output_get_2 (set `self.GameModeRef` _astetris_game_mode))
      (bind _output_get_3 (set `self.CurrentBlockSpeed` (`/Game/Core/Blueprints/TetrisGameMode.BlockSpeed` _output_get_2)))
      (`KismetSystemLibrary.PrintString` (`KismetStringLibrary.Concat_StrStr` "Current block speed :" (`KismetStringLibrary.Conv_DoubleToString` _output_get_3))))
    (:`then_1`
      ;[1 1 1] Move Peice Down Loop
      (`KismetSystemLibrary.K2_SetTimerDelegate` (delegate `Event MovePeiceDown`) (`self.CurrentBlockSpeed`) true))))

(event `Key|S`
  (params (Key :type "Key Structure"))
  (bind _returnvalue (`self.K2_GetActorLocation`))
  ;[1 1 1] Translate Blocks
  ;;[1 1 1] Translate X Front Back
  (:`Pressed`
    (if (not (`self.IsMoving`))
      (set `self.IsMoving` true)
      (set `self.DetectBoundryDirection` (100.0 0.0 0.0))
      (bind _canmoveoutput (`self.DetectBoundry`))
      (if _canmoveoutput
        (set `self.StartLocation` (`KismetMathLibrary.Vector_SnappedToGrid` _returnvalue (`self.PlayfieldCubeSize`)))
        (set `self.EndLocation` (`KismetMathLibrary.Vector_SnappedToGrid` (`KismetMathLibrary.MakeVector` (+ (.x _returnvalue) 100.0) (.y _returnvalue) (.z _returnvalue)) (`self.PlayfieldCubeSize`)))
        (bind (_direction _0_1) (`Timeline|Timeline_1` :!via `PlayFromStart`)
          (:`Update`
            (`self.K2_SetActorLocation` (`KismetMathLibrary.VLerp` (`self.StartLocation`) (`self.EndLocation`) _0_1)))
          (:`Finished`
            (set `self.IsMoving` false)))
        (else
          (set `self.IsMoving` false))))))

(event `Event MovePeiceDown`
  ;[1 1 1] Move Peice Down Loop
  (if (`self.IsMoving`)
    _
    (elif (`self.IsGameActive`)
      (set `self.IsMoving` true)
      (`self.MovePeiceDown`)
      (set `self.IsMoving` false))))

(event `Key|D`
  (params (Key :type "Key Structure"))
  (bind _returnvalue (`self.K2_GetActorLocation`))
  ;[1 1 1] Translate Blocks
  ;;[1 1 1] Translate Y (Left-Right)
  (:`Pressed`
    (if (not (`self.IsMoving`))
      (set `self.IsMoving` true)
      (set `self.DetectBoundryDirection` (0.0 -100.0 0.0))
      (bind _canmoveoutput (`self.DetectBoundry`))
      (if _canmoveoutput
        (set `self.StartLocation` (`KismetMathLibrary.Vector_SnappedToGrid` _returnvalue (`self.PlayfieldCubeSize`)))
        (set `self.EndLocation` (`KismetMathLibrary.Vector_SnappedToGrid` (`KismetMathLibrary.MakeVector` (.x _returnvalue) (- (.y _returnvalue) 100.0) (.z _returnvalue)) (`self.PlayfieldCubeSize`)))
        (bind (_direction _0_1) (`Timeline|Timeline_2` :!via `PlayFromStart`)
          (:`Update`
            (`self.K2_SetActorLocation` (`KismetMathLibrary.VLerp` (`self.StartLocation`) (`self.EndLocation`) _0_1)))
          (:`Finished`
            (set `self.IsMoving` false)))
        (else
          (set `self.IsMoving` false))))))

(event `Key|Down`
  (params (Key :type "Key Structure"))
  (bind _returnvalue (`self.K2_GetActorRotation`))
  ;[1 1 1] Rotation
  (:`Pressed`
    (if (not (`self.IsMoving`))
      (set `self.IsMoving` true)
      (`KismetSystemLibrary.PrintString` (`KismetStringLibrary.Conv_RotatorToString` _returnvalue) (`self.PrintDebugMovement`) true (struct :`R` 0.957218 :`G` 1.0 :`A` 1.0) 20.0)
      (set `self.StartingPeiceRotation` _returnvalue)
      (set `self.DetectBoundryDirection` (0.0 0.0 50.0))
      (set `self.PreviousTimelineValue` 0.0)
      (bind (_direction _pitch) (`Timeline|Timeline_7` :!via `PlayFromStart`)
        (:`Update`
          ;;[1 1 1] Timeline Body
          (`self.K2_AddActorWorldRotation` (`KismetMathLibrary.MakeRotator` 0.0 (- (`self.PreviousTimelineValue`) _pitch)))
          (bind _output_get (set `self.PreviousTimelineValue` _pitch))
          ;;[1 1 1] Boundry Flash on
          (bind _canmoveoutput (`self.DetectBoundryRotate`))
          (if (not _canmoveoutput)
            (`self.BoundryFlashOn`))
          ;;[1 1 1] Rotation value debug
          (`KismetSystemLibrary.PrintString` (`KismetStringLibrary.Conv_DoubleToString` _output_get) (`self.PrintDebugRotation`)))
        (:`Finished`
          (bind _canmoveoutput_2 (`self.DetectBoundryRotate`))
          (if _canmoveoutput_2
            (`KismetSystemLibrary.PrintString` "No Boundry Detected" (`self.PrintDebugRotation`) true (struct :`G` 1.0 :`B` 0.073006 :`A` 1.0) 20.0)
            (set `self.CurrentPeiceRotation` (`self.K2_GetActorRotation`))
            (set `self.IsMoving` false)
            (`self.BoundryFlashoff` :!label _label_2)
            (else
              (`KismetSystemLibrary.PrintString` "Boundry Detected" (`self.PrintDebugRotation`) true (struct :`R` 1.0 :`G` 0.059606 :`A` 1.0) 20.0)
              ;;[1 1 1] Animate undo Rotation
              (set `self.PreviousTimelineValue` 0.0)
              (bind (_direction_2 _yaw) (`Timeline|Timeline_5` :!via `PlayFromStart`)
                (:`Update`
                  ;;;[1 1 1] Timeline Body
                  (`self.K2_AddActorWorldRotation` (`KismetMathLibrary.MakeRotator` 0.0 (- _yaw (`self.PreviousTimelineValue`))))
                  (bind _output_get_2 (set `self.PreviousTimelineValue` _yaw))
                  (`KismetSystemLibrary.PrintString` (`KismetStringLibrary.Conv_DoubleToString` _output_get_2) (`self.PrintDebugRotation`) true (struct :`G` 0.66 :`B` 1.0 :`A` 1.0) 20.0))
                (:`Finished`
                  (set `self.CurrentPeiceRotation` (`self.StartingPeiceRotation`))
                  (set `self.IsMoving` false)
                  (goto _label_2))))))))))

(event `Key|A`
  (params (Key :type "Key Structure"))
  (bind _returnvalue (`self.K2_GetActorLocation`))
  ;[1 1 1] Translate Blocks
  ;;[1 1 1] Translate Y (Left-Right)
  (:`Pressed`
    (if (not (`self.IsMoving`))
      (set `self.IsMoving` true)
      (set `self.DetectBoundryDirection` (0.0 100.0 0.0))
      (bind _canmoveoutput (`self.DetectBoundry`))
      (if _canmoveoutput
        (set `self.StartLocation` (`KismetMathLibrary.Vector_SnappedToGrid` _returnvalue (`self.PlayfieldCubeSize`)))
        (set `self.EndLocation` (`KismetMathLibrary.Vector_SnappedToGrid` (`KismetMathLibrary.MakeVector` (.x _returnvalue) (+ (.y _returnvalue) 100.0) (.z _returnvalue)) (`self.PlayfieldCubeSize`)))
        (bind (_direction _0_1) (`Timeline|Timeline_3` :!via `PlayFromStart`)
          (:`Update`
            (`self.K2_SetActorLocation` (`KismetMathLibrary.VLerp` (`self.StartLocation`) (`self.EndLocation`) _0_1)))
          (:`Finished`
            (set `self.IsMoving` false)))
        (else
          (set `self.IsMoving` false))))))

(event `Key|P` :paused true
  (params (Key :type "Key Structure"))
  (bind _returnvalue (`GameplayStatics.GetPlayerController` 0))
  (bind _pausemenuref (`self.PauseMenuRef`))
  ;[1 1 1] Pause Menu Controls
  (:`Pressed`
    (`GameplayStatics.PlaySound2D` "/Game/Audio/SFX/Button/Window_Open_2.Window_Open_2" 1.0 1.0 0.0 null null :!label _label_3)
    (bind _returnvalue_2 (`GameplayStatics.SetGamePaused` (`self.Pause`)))
    (`KismetSystemLibrary.PrintString` (`KismetStringLibrary.Conv_BoolToString` _returnvalue_2) (`self.PauseDebug`))
    (`Widget.SetVisibility` _pausemenuref "Visible")
    (`/Game/Core/Blueprints/UserInterface/WBP_PauseMenu.On Paused` _pausemenuref)
    (`WidgetBlueprintLibrary.SetInputMode_UIOnlyEx` _returnvalue null)
    (set `PlayerController.bShowMouseCursor` true _returnvalue)))

(event `Key|Escape`
  (params (Key :type "Key Structure"))
  ;[1 1 1] Pause Menu Controls
  (:`Pressed`
    (goto _label_3)))

(event `Key|Left`
  (params (Key :type "Key Structure"))
  (bind _returnvalue (`self.K2_GetActorRotation`))
  ;[0.3873 1 0.4415] Rotate Yaw
  ;;[1 1 1] Left
  (:`Pressed`
    (if (not (`self.IsMoving`))
      (set `self.IsMoving` true)
      (`KismetSystemLibrary.PrintString` (`KismetStringLibrary.Conv_RotatorToString` _returnvalue) (`self.PrintDebugMovement`) true (struct :`R` 0.957218 :`G` 1.0 :`A` 1.0) 20.0)
      (set `self.StartingPeiceRotation` _returnvalue)
      (set `self.DetectBoundryDirection` (0.0 50.0 0.0))
      (set `self.PreviousTimelineValue` 0.0)
      (bind (_direction _yaw) (`Timeline|Timeline_8` :!via `PlayFromStart`)
        (:`Update`
          ;;;[1 1 1] Timeline Body
          (`self.K2_AddActorWorldRotation` (`KismetMathLibrary.MakeRotator` 0.0 0.0 (- _yaw (`self.PreviousTimelineValue`))))
          (set `self.PreviousTimelineValue` _yaw)
          ;;;[1 1 1] Boundry Flash on
          (bind _canmoveoutput (`self.DetectBoundryRotate`))
          (if (not _canmoveoutput)
            (`KismetSystemLibrary.PrintString` "Boundry Detected" (`self.PrintDebugRotation`) true (struct :`R` 0.135237 :`G` 1.0 :`A` 1.0) 20.0)
            (`self.BoundryFlashOn`)))
        (:`Finished`
          (bind _canmoveoutput_2 (`self.DetectBoundryRotate`))
          (if _canmoveoutput_2
            (`KismetSystemLibrary.PrintString` "No Boundry Detected" (`self.PrintDebugRotation`) true (struct :`G` 1.0 :`B` 0.073006 :`A` 1.0) 20.0)
            (set `self.CurrentPeiceRotation` (`self.K2_GetActorRotation`))
            (set `self.IsMoving` false)
            (`self.BoundryFlashoff` :!label _label_4)
            (else
              (`KismetSystemLibrary.PrintString` "Boundry Detected" (`self.PrintDebugRotation`) true (struct :`R` 1.0 :`G` 0.059606 :`A` 1.0) 20.0)
              ;;;[1 1 1] Animate undo Rotation
              (set `self.PreviousTimelineValue` 0.0)
              (bind (_direction_2 _yaw_2) (`Timeline|Timeline` :!via `PlayFromStart`)
                (:`Update`
                  ;;;;[1 1 1] Timeline Body
                  (`self.K2_AddActorWorldRotation` (`KismetMathLibrary.MakeRotator` 0.0 0.0 (- (`self.PreviousTimelineValue`) _yaw_2)))
                  (bind _output_get (set `self.PreviousTimelineValue` _yaw_2))
                  (`KismetSystemLibrary.PrintString` (`KismetStringLibrary.Conv_DoubleToString` _output_get) (`self.PrintDebugRotation`) true (struct :`G` 0.66 :`B` 1.0 :`A` 1.0) 20.0))
                (:`Finished`
                  (set `self.CurrentPeiceRotation` (`self.StartingPeiceRotation`))
                  (set `self.IsMoving` false)
                  (goto _label_4))))))))))

(event `Key|Right`
  (params (Key :type "Key Structure"))
  (bind _returnvalue (`self.K2_GetActorRotation`))
  ;[0.3873 1 0.4415] Rotate Yaw
  ;;[1 1 1] Right
  (:`Pressed`
    (if (not (`self.IsMoving`))
      (set `self.IsMoving` true)
      (`KismetSystemLibrary.PrintString` (`KismetStringLibrary.Conv_RotatorToString` _returnvalue) false (`self.PrintDebugMovement`) (struct :`R` 0.957218 :`G` 1.0 :`A` 1.0) 20.0)
      (set `self.StartingPeiceRotation` _returnvalue)
      (set `self.DetectBoundryDirection` (0.0 -50.0 0.0))
      (set `self.PreviousTimelineValue` 0.0)
      (bind (_direction _pitch) (`Timeline|Timeline_9` :!via `PlayFromStart`)
        (:`Update`
          ;;;[1 1 1] Timeline Body
          (`self.K2_AddActorWorldRotation` (`KismetMathLibrary.MakeRotator` 0.0 0.0 (- (`self.PreviousTimelineValue`) _pitch)))
          (bind _output_get (set `self.PreviousTimelineValue` _pitch))
          ;;;[1 1 1] Boundry Flash on
          (bind _canmoveoutput (`self.DetectBoundry`))
          (if (not _canmoveoutput)
            (`self.BoundryFlashOn`))
          ;;;[1 1 1] Rotation value debug
          (`KismetSystemLibrary.PrintString` (`KismetStringLibrary.Conv_DoubleToString` _output_get) (`self.PrintDebugRotation`)))
        (:`Finished`
          (bind _canmoveoutput_2 (`self.DetectBoundry`))
          (if _canmoveoutput_2
            (`KismetSystemLibrary.PrintString` "No Boundry Detected" (`self.PrintDebugMovement`) true (struct :`G` 1.0 :`B` 0.073006 :`A` 1.0) 20.0)
            (set `self.CurrentPeiceRotation` (`self.K2_GetActorRotation`))
            (set `self.IsMoving` false)
            (`self.BoundryFlashoff` :!label _label_5)
            (else
              ;;;[1 1 1] Animate undo Rotation
              (set `self.PreviousTimelineValue` 0.0)
              (bind (_direction_2 _yaw) (`Timeline|Timeline_4` :!via `PlayFromStart`)
                (:`Update`
                  ;;;;[1 1 1] Timeline Body
                  (`self.K2_AddActorWorldRotation` (`KismetMathLibrary.MakeRotator` 0.0 0.0 (- _yaw (`self.PreviousTimelineValue`))))
                  (bind _output_get_2 (set `self.PreviousTimelineValue` _yaw))
                  (`KismetSystemLibrary.PrintString` (`KismetStringLibrary.Conv_DoubleToString` _output_get_2) false true (struct :`G` 0.66 :`B` 1.0 :`A` 1.0) 20.0))
                (:`Finished`
                  (set `self.CurrentPeiceRotation` (`self.StartingPeiceRotation`))
                  (set `self.IsMoving` false)
                  (goto _label_5))))))))))

(fn `BoundryFlashoff`
  (bind _startingmat (`self.StartingMat`))
  (for _array_element (`self.K2_GetComponentsByClass` "/Script/Engine.StaticMeshComponent")
    (`PrimitiveComponent.SetMaterial` _array_element 0 _startingmat)
    (`KismetSystemLibrary.PrintString` (`KismetSystemLibrary.GetDisplayName` _startingmat) (`self.PrintDebugOther`) true (struct :`R` 0.156562 :`B` 1.0 :`A` 1.0))))

(fn `BoundryFlashOn`
  (for _array_element (`self.K2_GetComponentsByClass` "/Script/Engine.StaticMeshComponent")
    (`PrimitiveComponent.SetMaterial` _array_element 0 "/Game/Core/Materials/Color/MI_Collision_Red.MI_Collision_Red")))

(fn `DetectBoundry`
  (returns (CanMoveOutput :type Boolean))
  (locals (CanMove :type Boolean :default true))
  ;[1 1 1] Set Linetrace draw debug type
  (bind _returnvalue (`GameplayStatics.GetCurrentLevelName` true))
  (if (`KismetStringLibrary.EqualEqual_StrStr` _returnvalue "MenuLevel")
    (set `self.Draw Debug Type` "None")
    (else
      (set `self.Draw Debug Type` "None")))
  (for _array_element (`self.K2_GetComponentsByClass` "/Script/Engine.StaticMeshComponent")
    (bind _returnvalue_2 (`SceneComponent.K2_GetComponentLocation` _array_element))
    (bind (_outhits _returnvalue_3) (`KismetSystemLibrary.LineTraceMulti` :`Start` _returnvalue_2 :`End` (+ _returnvalue_2 (`self.DetectBoundryDirection`)) :`TraceChannel` "TraceTypeQuery1" :`DrawDebugType` (`self.Draw Debug Type`)))
    (for _array_element_2 _outhits
      (`KismetSystemLibrary.PrintString` (`KismetSystemLibrary.GetDisplayName` (`.HitActor` (`GameplayStatics.BreakHitResult` _array_element_2))) (`self.PrintDebugCollision`)))
    (if _returnvalue_3
      (set `local.CanMove` false)))
  (return (`local.CanMove`)))

(fn `DetectBoundryRotate`
  (returns (CanMoveOutput :type Boolean))
  (locals (CanMove :type Boolean :default true))
  ;[1 1 1] Set Linetrace Visibility
  (bind _returnvalue (`GameplayStatics.GetCurrentLevelName` true))
  (if (`KismetStringLibrary.EqualEqual_StrStr` _returnvalue "MenuLevel")
    (set `self.Draw Debug Type` "None")
    (else
      (set `self.Draw Debug Type` "None")))
  (for _array_element (`self.K2_GetComponentsByClass` "/Script/Engine.StaticMeshComponent")
    (bind _returnvalue_2 (`SceneComponent.K2_GetComponentLocation` _array_element))
    (bind (_outhits _returnvalue_3) (`KismetSystemLibrary.LineTraceMulti` :`Start` _returnvalue_2 :`End` (+ _returnvalue_2 (`self.DetectBoundryDirection`)) :`TraceChannel` "TraceTypeQuery1" :`DrawDebugType` (`self.Draw Debug Type`)))
    (for _array_element_2 _outhits
      (`KismetSystemLibrary.PrintString` (`KismetSystemLibrary.GetDisplayName` (`.HitActor` (`GameplayStatics.BreakHitResult` _array_element_2))) (`self.PrintDebugCollision`)))
    (if _returnvalue_3
      (set `local.CanMove` false)))
  (return (`local.CanMove`)))

(fn `EndGame`
  (set `self.IsGameActive` false)
  (`KismetSystemLibrary.PrintString` "Game Over" (`self.PrintDebugOther`))
  (bind _returnvalue (`|CreateWidget` "/Game/Core/Blueprints/UserInterface/WBP_EndGameMenu.WBP_EndGameMenu_C"))
  (`UserWidget.AddToViewport` _returnvalue 0))

(fn `GetStartingMat`
  (for _array_element (`self.K2_GetComponentsByClass` "/Script/Engine.StaticMeshComponent")
    (bind _output_get (set `self.StartingMat` (`PrimitiveComponent.GetMaterial` _array_element 0)))
    (`KismetSystemLibrary.PrintString` (`KismetSystemLibrary.GetDisplayName` _output_get) (`self.PrintDebugOther`))
    (break)))

(fn `MovePeiceDown`
  (bind _returnvalue_location (`KismetMathLibrary.BreakTransform` (`self.GetTransform`)))
  ;[1 1 1] Move Peice Down
  (set `self.DetectBoundryDirection` (0.0 0.0 -100.0))
  (bind _canmoveoutput (`self.DetectBoundry`))
  (if _canmoveoutput
    (`self.CallTimeline` _returnvalue_location (`KismetMathLibrary.MakeVector` (.x _returnvalue_location) (.y _returnvalue_location) (- (.z _returnvalue_location) 100.0)))
    (else
      (`self.SpawnCubes`)
      (set `self.IsMoving` false)
      (bind _astetris_game_mode (cast `/Game/Core/Blueprints/TetrisGameMode` (`GameplayStatics.GetGameMode`)))
      (`self.K2_DestroyActor`)
      (if (>= (.z (`self.K2_GetActorLocation`)) (.z (.location (`self.GetTransform` (`/Game/Core/Blueprints/TetrisGameMode.PeicesSpawnPoint` _astetris_game_mode)))))
        (`self.EndGame`)
        (else
          (`/Game/Core/Blueprints/TetrisGameMode.SpawnNewPeice` :`self` _astetris_game_mode))))))

(fn `SpawnCubes`
  (bind _returnvalue (`GameplayStatics.GetActorOfClass` "/Game/Core/Blueprints/Fiverr/Bp_GridManager.Bp_GridManager_C"))
  (if (`KismetStringLibrary.EqualEqual_StrStr` (`self.CurrentLevel`) "MenuLevel")
    ;[1 1 1] This doesnt spawn the entire shape, it loops through the individual boxes that make up the tertris pecies, spawns a new one at the same transform as the previous.
    (for _array_element (`self.K2_GetComponentsByClass` "/Script/Engine.StaticMeshComponent")
      (if (not (== _array_element null))
        (`|SpawnActorFromClass` "/Game/Core/Blueprints/BP_Cubes.BP_Cubes_C" (`KismetMathLibrary.Conv_VectorToTransform` (- (`SceneComponent.K2_GetComponentLocation` _array_element) (0.0 0.0 0.0))) "Undefined" "MultiplyWithRoot" null (`PrimitiveComponent.GetMaterial` _array_element 0) (struct) null)))
    (elif (`self.IsMoving`)
      (`/Game/Core/Blueprints/Fiverr/Bp_GridManager.Place Piece on Grid` _returnvalue self)
      (else
        (`/Game/Core/Blueprints/Fiverr/Bp_GridManager.Place Piece on Grid` _returnvalue self)))))

(fn `UserConstructionScript`)