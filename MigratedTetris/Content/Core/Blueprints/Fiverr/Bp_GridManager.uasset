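; Grid manager actor for a 3D Tetris-style game, storing landed cubes in a PlacedBlocks map keyed by integer grid position.
; Landed pieces are split into snapped BP_Cubes, then the affected Z layers are checked and full ones cleared.
; After a clear, flood fill finds six-way connected groups and drops unsupported ones cell by cell until settled.
; Placements without a clear and each cleared layer add score, printed for debug.
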(event `self.ReceiveBeginPlay`
  ;[1 1 1] Debug on event begin play, fill 10 x 9 blocks with a cube
)

(fn `ApplyGroupGravity`
  (locals (MovedAnyGroup :type Boolean) (CheckedBlocks :type "Array of /Game/Core/Blueprints/BP_Cubes Object Reference") (CurrentGroup :type "Array of /Game/Core/Blueprints/BP_Cubes Object Reference"))
  ;[0.005737 0 0.5052] APPLY GROUP GRAVITY
  ;
  ; Applies gravity to all placed blocks after layers are cleared.
  ;
  ; The function loops through the current PlacedBlocks map and finds connected block groups. Each group is only checked once by storing already checked blocks in CheckedBlocks.
  ;
  ; If a group is not supported by the floor or another block, it is moved down by one grid cell and the gravity check starts again. This repeats until no group was moved anymore, meaning all remaining blocks are resting correctly.
  (for _ (range 51)
    (set `local.MovedAnyGroup` false)
    (`KismetArrayLibrary.Array_Clear` (`local.CheckedBlocks`))
    (bind _keys (`BlueprintMapLibrary.Map_Keys` (`self.PlacedBlocks`)))
    (for _array_element _keys
      (bind _value (`BlueprintMapLibrary.Map_Find` (`self.PlacedBlocks`) _array_element))
      (if (not (`KismetArrayLibrary.Array_Contains` (`local.CheckedBlocks`) _value))
        (bind _connectedblocks (`self.FindConnectedGroup` _value))
        (`KismetArrayLibrary.Array_Append` (`local.CheckedBlocks`) _connectedblocks)
        (bind _issupported (`self.IsGroupSupported` _connectedblocks))
        (if (not _issupported)
          (`self.MoveGroupDownOne` _connectedblocks)
          (set `local.MovedAnyGroup` true)
          (break))))
    (if (not (`local.MovedAnyGroup`))
      (break))))

(fn `CheckLayers`
  (params (LayersToCheck :type "Array of Integer"))
  (locals (EmptyField :type Boolean) (CurrentZ :type Integer) (CurrentX :type Integer) (CompletedLayers :type "Array of Integer"))
  ;[0 0.02029 0.4271] CHECK LAYERS
  ;
  ; Checks if any affected grid layers are completely filled.
  ;
  ; For each layer passed into the function, the system loops through every X and Y position of the 10x10 grid and checks if a block exists in the PlacedBlocks map.
  ;
  ; If every cell in that layer is occupied, the layer is added to the CompletedLayers list. After all layers are checked, completed layers are cleared and gravity is applied to the remaining blocks.
  (for _array_element LayersToCheck
    (set `local.CurrentZ` _array_element)
    (set `local.EmptyField` false)
    (for _index (range (`self.GridSizeX`))
      (if (`local.EmptyField`)
        (break)
        (else
          (set `local.CurrentX` _index)
          (for _index_2 (range (`self.GridSizeY`))
            (if (not (`BlueprintMapLibrary.Map_Contains` (`self.PlacedBlocks`) (make `IntVector` (`local.CurrentX`) _index_2 (`local.CurrentZ`))))
              (set `local.EmptyField` true)
              (break))))))
    (if (not (`local.EmptyField`))
      (`KismetArrayLibrary.Array_Add` (`local.CompletedLayers`) (`local.CurrentZ`))))
  (if (> (`KismetArrayLibrary.Array_Length` (`local.CompletedLayers`)) 0)
    (`self.ClearLayers` (`local.CompletedLayers`))
    (`self.ApplyGroupGravity`)
    (else
      (`self.ScoreBlock`))))

(fn `ClearLayers`
  (params (LayersToClear :type "Array of Integer"))
  ;[0 0.1367 0.6562] CLEAR LAYERS
  ;
  ; Removes all blocks from completed layers.
  ;
  ; For each completed layer, the function loops through every X and Y cell in the grid and builds the matching grid position. If a block exists at that position in the PlacedBlocks map, the block actor is destroyed and the map entry is removed.
  ;
  ; This clears the full 10x10x1 layer from both the level and the grid data.
  (for _array_element LayersToClear
    (`self.ScoreTetris`)
    (for _index (range (`self.GridSizeX`))
      (for _index_2 (range (`self.GridSizeY`))
        (bind _intvector (make `IntVector` _index _index_2 _array_element))
        (`self.K2_DestroyActor` (`BlueprintMapLibrary.Map_Find` (`self.PlacedBlocks`) _intvector))
        (`BlueprintMapLibrary.Map_Remove` (`self.PlacedBlocks`) _intvector)))))

(fn `FindConnectedGroup`
  (params (PlacedBlock :type "/Game/Core/Blueprints/BP_Cubes Object Reference"))
  (returns (ConnectedBlocks :type "Array of /Game/Core/Blueprints/BP_Cubes Object Reference"))
  (locals (`Open List` :type "Array of /Game/Core/Blueprints/BP_Cubes Object Reference") (`Connected Blocks Local` :type "Array of /Game/Core/Blueprints/BP_Cubes Object Reference") (`Visited Positions` :type "Array of IntVector Structure") (CurrentBlock :type "/Game/Core/Blueprints/BP_Cubes Object Reference"))
  (bind _gridposition (`/Game/Core/Blueprints/BP_Cubes.GridPosition` (`local.CurrentBlock`)))
  ;[0 0.01541 0.6094] FIND CONNECTED GROUP - SEARCH SETUP
  ;
  ; Finds all blocks that are directly connected to the starting block.
  ;
  ; The function uses an OpenList to store blocks that still need to be checked and a VisitedPositions list to avoid checking the same grid position multiple times. Each checked block is added to the ConnectedBlocks list.
  (`KismetArrayLibrary.Array_Add` (`local.Open List`) PlacedBlock)
  (for _ (range 501)
    (if (<= (`KismetArrayLibrary.Array_Length` (`local.Open List`)) 0)
      (break)
      (else
        (set `local.CurrentBlock` (`|GetArrayItem` (`local.Open List`)))
        (`KismetArrayLibrary.Array_Remove` (`local.Open List`))
        (if (not (`KismetArrayLibrary.Array_Contains` (`local.Visited Positions`) _gridposition))
          (`KismetArrayLibrary.Array_Add` (`local.Visited Positions`) _gridposition)
          (`KismetArrayLibrary.Array_Add` (`local.Connected Blocks Local`) (`local.CurrentBlock`))
          ;;[0 0.2083 0.02245] NEIGHBOR CHECK
          ;;
          ;; Gets all neighboring grid positions around the current block.
          ;;
          ;; For each neighbor, the function checks if a placed block exists at that position. If the neighbor was not already visited and is not already in the OpenList, it gets added to the OpenList so it can be checked later.
          ;;
          ;; This continues until there are no more connected blocks left to check.
          (bind _neighborpositions (`self.GetNeighborPositions` _gridposition))
          (for _array_element _neighborpositions
            (bind (_value _returnvalue) (`BlueprintMapLibrary.Map_Find` (`self.PlacedBlocks`) _array_element))
            (if _returnvalue
              (if (and (not (`KismetArrayLibrary.Array_Contains` (`local.Connected Blocks Local`) _value)) (not (`KismetArrayLibrary.Array_Contains` (`local.Open List`) _value)))
                (`KismetArrayLibrary.Array_Add` (`local.Open List`) _value))))))))
  (return (`local.Connected Blocks Local`)))

(fn `GetNeighborPositions`
  (params (GridPosition :type "IntVector Structure"))
  (returns (NeighborPositions :type "Array of IntVector Structure"))
  (locals (NeighbourPositions :type "Array of IntVector Structure"))
  (bind (_x _y _z) (break `IntVector` GridPosition))
  (bind (_x_2 _y_2 _z_2) (break `IntVector` GridPosition))
  (bind (_x_3 _y_3 _z_3) (break `IntVector` GridPosition))
  (bind (_x_4 _y_4 _z_4) (break `IntVector` GridPosition))
  (bind (_x_5 _y_5 _z_5) (break `IntVector` GridPosition))
  (bind (_x_6 _y_6 _z_6) (break `IntVector` GridPosition))
  (bind _neighbourpositions (`local.NeighbourPositions`))
  ;[0.01987 0 0.5] GET NEIGHBOR POSITIONS
  ;
  ; Returns the six grid positions directly next to the given block position.
  ;
  ; The function creates neighbor positions for left, right, forward, backward, above, and below by adding or subtracting 1 from the X, Y, or Z grid coordinate.
  ;
  ; These positions are used by FindConnectedGroup to check which blocks are connected.
  (`KismetArrayLibrary.Array_Add` _neighbourpositions (make `IntVector` (+ _x_3 1) _y_3 _z_3))
  (`KismetArrayLibrary.Array_Add` _neighbourpositions (make `IntVector` (+ _x_4 -1) _y_4 _z_4))
  (`KismetArrayLibrary.Array_Add` _neighbourpositions (make `IntVector` _x_5 (+ _y_5 1) _z_5))
  (`KismetArrayLibrary.Array_Add` _neighbourpositions (make `IntVector` _x_6 (+ _y_6 -1) _z_6))
  (`KismetArrayLibrary.Array_Add` _neighbourpositions (make `IntVector` _x_2 _y_2 (+ _z_2 1)))
  (`KismetArrayLibrary.Array_Add` _neighbourpositions (make `IntVector` _x _y (+ _z -1)))
  (return (`local.NeighbourPositions`)))

(fn `GridToWorld`
  (params (GridPosition :type "IntVector Structure"))
  (returns (WorldLocation :type "Vector Structure"))
  (bind (_x _y _z) (break `IntVector` GridPosition))
  (bind _blocksize (`self.BlockSize`))
  (bind (_returnvalue_x _returnvalue_y _returnvalue_z) (`KismetMathLibrary.BreakVector` (`SceneComponent.K2_GetComponentLocation` (`self.DefaultSceneRoot`))))
  ;[0.006899 0 0.4427] GRID TO WORLD
  ;
  ; Converts an IntVector grid position back into a world location.
  ;
  ; Each grid coordinate is multiplied by BlockSize to convert grid cells into Unreal world units. The GridManager's world location is then added as the grid origin.
  ;
  ; The Z value also adds one BlockSize offset, so grid layer 1 sits above the floor instead of at world Z = 0.
  (return (`KismetMathLibrary.MakeVector` (+ (* _x _blocksize) _returnvalue_x) (+ (* _y _blocksize) _returnvalue_y) (+ (* _z _blocksize) _returnvalue_z))))

(fn `IsGroupSupported`
  (params (ConnectedBlocks :type "Array of /Game/Core/Blueprints/BP_Cubes Object Reference"))
  (returns (IsSupported :type Boolean))
  ;[0 0.08144 0.5885] IS GROUP SUPPORTED
  ;
  ; Checks if a connected block group is currently supported.
  ;
  ; Each block in the group is checked. If any block is on the floor layer, the whole group is supported. Otherwise, the function checks the grid cell directly below each block.
  ;
  ; If there is another placed block below the group, and that block is not part of the same group, the group is supported. If no support is found, the group can fall down.
  (for _array_element ConnectedBlocks
    (bind (_x _y _z) (break `IntVector` (`/Game/Core/Blueprints/BP_Cubes.GridPosition` _array_element)))
    (if (<= _z (`self.FloorZ`))
      (return true)
      (else
        (bind (_value _returnvalue) (`BlueprintMapLibrary.Map_Find` (`self.PlacedBlocks`) (make `IntVector` _x _y (+ _z -1))))
        (if _returnvalue
          (if (not (`KismetArrayLibrary.Array_Contains` (`local.ConnectedBlocks`) _value))
            (return true))))))
  (return false))

(fn `MoveGroupDownOne`
  (params (ConnectedBlocks :type "Array of /Game/Core/Blueprints/BP_Cubes Object Reference"))
  (locals (OldPos :type "IntVector Structure") (CurrentBlock :type "/Game/Core/Blueprints/BP_Cubes Object Reference") (NewPos :type "IntVector Structure"))
  ;[0 0.06143 0.4479] MOVE GROUP DOWN ONE
  ;
  ; Moves a connected block group down by one grid cell.
  ;
  ; The function first checks if any block in the group is already on the floor. If so, the group is not moved.
  ;
  ; Before moving the blocks, their old positions are removed from the PlacedBlocks map. Then each block gets a new grid position with Z - 1, is moved to the matching world location, and is added back into the map with its updated position.
  (for _array_element ConnectedBlocks
    (if (<= (`.Z` (break `IntVector` (`/Game/Core/Blueprints/BP_Cubes.GridPosition` _array_element))) (`self.FloorZ`))
      (return)))
  (for _array_element_2 (`local.ConnectedBlocks`)
    (set `local.OldPos` (`/Game/Core/Blueprints/BP_Cubes.GridPosition` _array_element_2))
    (`BlueprintMapLibrary.Map_Remove` (`self.PlacedBlocks`) (`local.OldPos`)))
  (for _array_element_3 (`local.ConnectedBlocks`)
    (set `local.CurrentBlock` _array_element_3)
    (bind (_x _y _z) (break `IntVector` (`/Game/Core/Blueprints/BP_Cubes.GridPosition` _array_element_3)))
    (set `local.NewPos` (make `IntVector` _x _y (- _z 1)))
    (set `/Game/Core/Blueprints/BP_Cubes.GridPosition` (`local.NewPos`) (`local.CurrentBlock`))
    (bind _worldlocation (`self.GridToWorld` (`local.NewPos`)))
    (`self.K2_SetActorLocation` (`local.CurrentBlock`) _worldlocation false true)
    (`BlueprintMapLibrary.Map_Add` (`self.PlacedBlocks`) (`/Game/Core/Blueprints/BP_Cubes.GridPosition` (`local.CurrentBlock`)) (`local.CurrentBlock`))))

(fn `Place Piece on Grid`
  (params (Piece :type "Actor Object Reference"))
  (locals (ModifiedZlayers :type "Array of Integer"))
  ;[0 0.07503 0.5625] PLACE PIECE ON GRID
  ;
  ; Registers a landed piece into the grid system.
  ;
  ; The function loops through all cube components of the placed piece, converts each cube's world location into a grid position, and snaps it to the grid. It then spawns a separate placed block actor at that position and adds it to the PlacedBlocks map.
  ;
  ; After all cubes are registered, the original falling piece is destroyed and the affected layers are checked for completion.
  (for _array_element (`self.K2_GetComponentsByClass` Piece "/Script/Engine.StaticMeshComponent")
    (bind _gridpostion (`self.WorldToGrid` (`SceneComponent.K2_GetComponentLocation` _array_element)))
    (`KismetArrayLibrary.Array_AddUnique` (`local.ModifiedZlayers`) (`.Z` (break `IntVector` _gridpostion)))
    (bind _worldlocation (`self.GridToWorld` _gridpostion))
    (bind _returnvalue (`|SpawnActorFromClass` "/Game/Core/Blueprints/BP_Cubes.BP_Cubes_C" (`KismetMathLibrary.MakeTransform` _worldlocation) "Undefined" "MultiplyWithRoot" null (`PrimitiveComponent.GetMaterial` _array_element 0) _gridpostion null))
    (`BlueprintMapLibrary.Map_Add` (`self.PlacedBlocks`) _gridpostion _returnvalue))
  (`self.K2_DestroyActor` Piece)
  (`self.CheckLayers` (`local.ModifiedZlayers`)))

(fn `ScoreBlock`
  (bind _output_get (set `self.CurrentScore` (+ 100 (`self.CurrentScore`))))
  (`KismetSystemLibrary.PrintString` (`KismetStringLibrary.Concat_StrStr` "Score Block! CurrentScore: " (`KismetStringLibrary.Conv_IntToString` _output_get))))

(fn `ScoreTetris`
  (bind _output_get (set `self.CurrentScore` (+ 500 (`self.CurrentScore`))))
  (`KismetSystemLibrary.PrintString` (`KismetStringLibrary.Concat_StrStr` "Score Tetris! CurrentScore: " (`KismetStringLibrary.Conv_IntToString` _output_get))))

(fn `UserConstructionScript`)

(fn `WorldToGrid`
  (params (WorldLocation :type "Vector Structure"))
  (returns (GridPostion :type "IntVector Structure"))
  (bind (_returnvalue_x _returnvalue_y _returnvalue_z) (`KismetMathLibrary.BreakVector` (- WorldLocation (`self.K2_GetActorLocation`))))
  ;[0 0.01136 0.4896] WORLD TO GRID
  ;
  ; Converts a world location into a grid position.
  ;
  ; First, the GridManager's world location is subtracted from the input location, so the grid is calculated relative to this actor. Then the result is divided by BlockSize to convert Unreal units into grid cells.
  ;
  ; The values are rounded to the nearest whole number and returned as an IntVector, which is used as the key for the PlacedBlocks map.
  (return (make `IntVector` (`KismetMathLibrary.Round` (/ _returnvalue_x (`self.BlockSize`))) (`KismetMathLibrary.Round` (/ _returnvalue_y (`self.BlockSize`))) (`KismetMathLibrary.Round` (/ _returnvalue_z (`self.BlockSize`))))))