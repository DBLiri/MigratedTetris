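; BP_ScoreManager records the components detected by line traces cast from its own static mesh components; no score is calculated here.
; Each Tick, every mesh fires a debug-drawn multi line trace on Visibility along world +X.
; Newly hit components are added once to CurrentHitList and printed, and nothing removes them.
; A looping timer started on BeginPlay periodically prints the whole list to screen.
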(event `self.ReceiveBeginPlay`
  (`KismetSystemLibrary.K2_SetTimerDelegate` (delegate `print array`) 2.0 true))

(event `print array`
  (for _array_element (`self.CurrentHitList`)
    (`KismetSystemLibrary.PrintString` (`KismetSystemLibrary.GetDisplayName` _array_element))))

(event `self.ReceiveTick`
  (params (DeltaSeconds :type "Float (single-precision)"))
  (for _array_element (`self.K2_GetComponentsByClass` "/Script/Engine.StaticMeshComponent")
    (bind _returnvalue (`SceneComponent.K2_GetComponentLocation` _array_element))
    (bind _outhits (`KismetSystemLibrary.LineTraceMulti` _returnvalue (+ _returnvalue (10000.0 0.0 0.0)) "TraceTypeQuery1" false (`self.ActorsToIgnore`) "ForDuration"))
    (for _array_element_2 _outhits
      (bind (_bblockinghit _binitialoverlap _time _distance _location _impactpoint _normal _impactnormal _physmat _hitactor _hitcomponent) (`GameplayStatics.BreakHitResult` _array_element_2))
      (if (== (`KismetArrayLibrary.Array_Find` (`self.CurrentHitList`) _hitcomponent) -1)
        (`KismetArrayLibrary.Array_Add` (`self.CurrentHitList`) _hitcomponent)
        (`KismetSystemLibrary.PrintString` (`KismetSystemLibrary.GetDisplayName` _hitcomponent))))))

(fn `UserConstructionScript`)