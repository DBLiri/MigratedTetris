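; BP_CameraSwitcher cycles the player's view around a board by moving the player pawn between preset camera points.
; E and Q call MoveRight and MoveLeft, which step the index backward and forward through CameraLocations with wraparound.
; SetLocation, also run on BeginPlay, snaps the pawn to that point and turns control rotation toward BoardTargetPoint.
; A Timeline-based transform lerp exists in CustomEvent2, but its only call is disconnected.
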(event `self.ReceiveBeginPlay`
  (`GameplayStatics.SetViewportMouseCaptureMode` "NoCapture")
  (`self.EnableInput` (`GameplayStatics.GetPlayerController` 0))
  (`self.SetLocation`)
  (`KismetSystemLibrary.PrintString` "222"))

(event `CustomEvent2`
  (params (StartLocation :type "Transform Structure") (EndLocation :type "Transform Structure"))
  (bind (_direction _cameramovetrack) (`Timeline|Timeline` :!via `PlayFromStart`)
    (:`Update`
      (`self.K2_SetActorTransform` (`GameplayStatics.GetPlayerPawn` 0) (`KismetMathLibrary.TLerp` StartLocation EndLocation _cameramovetrack) false false))
    (:`Finished`
      (`KismetSystemLibrary.PrintString` "Hello"))))

(event `Key|E`
  (params (Key :type "Key Structure"))
  (:`Pressed`
    (`self.MoveRight`)))

(event `Key|Q`
  (params (Key :type "Key Structure"))
  (:`Pressed`
    (`self.MoveLeft`)))

(fn `MoveLeft`
  (bind _returnvalue (+ (`self.CurrentCameraIndex`) 1))
  (set `self.CurrentCameraIndex` (`KismetMathLibrary.SelectInt` 0 _returnvalue (> _returnvalue (- (`KismetArrayLibrary.Array_Length` (`self.CameraLocations`)) 1))))
  (`self.SetLocation`))

(fn `MoveRight`
  (bind _returnvalue (- (`self.CurrentCameraIndex`) 1))
  (set `self.CurrentCameraIndex` (`KismetMathLibrary.SelectInt` (- (`KismetArrayLibrary.Array_Length` (`self.CameraLocations`)) 1) _returnvalue (< _returnvalue 0)))
  (`self.SetLocation`))

(fn `SetLocation`
  (bind _returnvalue_location (`KismetMathLibrary.BreakTransform` (`self.GetTransform` (`self.BoardTargetPoint`))))
  (bind (_returnvalue_location_2 _returnvalue_rotation _returnvalue_scale) (`KismetMathLibrary.BreakTransform` (`self.GetTransform` (`|GetArrayItem` (`self.CameraLocations`) (`self.CurrentCameraIndex`)))))
  ;[1 0.9871 0] When called set the tranform of the camera to the index of the target point in the array, then force the pawn to look at board
  (`self.K2_SetActorTransform` (`GameplayStatics.GetPlayerPawn` 0) (`KismetMathLibrary.MakeTransform` _returnvalue_location_2 _returnvalue_rotation _returnvalue_scale) false false)
  (`Controller.SetControlRotation` (`PlayerState.GetPlayerController` (`Pawn.PlayerState` (`GameplayStatics.GetPlayerPawn` 0))) (`KismetMathLibrary.FindLookAtRotation` (`self.K2_GetActorLocation` (`GameplayStatics.GetPlayerPawn` 0)) _returnvalue_location)))

(fn `UserConstructionScript`)