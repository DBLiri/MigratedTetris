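; Main menu mode Blueprint that keeps spawning random Tetris pieces in the level while it runs.
; BeginPlay starts a looping one-second timer that calls SpawnPeiceRandom.
; Each call gathers all TargetPoint actors, then spawns a random class from the TetrrisPecies array at a random point's transform.
; Spawning adjusts for collisions but always succeeds, and nothing here removes the spawned pieces.
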(event `self.ReceiveBeginPlay`
  (`KismetSystemLibrary.K2_SetTimerDelegate` (delegate `Spawn Peice`) 1.0 true))

(event `Spawn Peice`
  (`self.SpawnPeiceRandom`))

(fn `SpawnPeiceRandom`
  (bind _tetrrispecies (`self.TetrrisPecies`))
  (bind _outactors (`GameplayStatics.GetAllActorsOfClass` "/Script/Engine.TargetPoint"))
  (bind _output_get (set `self.TargetPoints` _outactors))
  (`|SpawnActorFromClass` (`|GetArrayItem` _tetrrispecies (`KismetMathLibrary.RandomIntegerInRange` 0 (`KismetArrayLibrary.Array_LastIndex` _tetrrispecies))) (`self.GetTransform` (`|GetArrayItem` (`self.TargetPoints`) (`KismetMathLibrary.RandomIntegerInRange` 0 (`KismetArrayLibrary.Array_LastIndex` _output_get)))) "AdjustIfPossibleButAlwaysSpawn" "MultiplyWithRoot" null null)
  (return))

(fn `UserConstructionScript`)