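; BP_Playfeild is a cube piece of the playfield, apparently for a Tetris-style game, with no active gameplay logic.
; Its construction script disables Nanite on the Cube component, assigns a box mesh and uses the EdgePeice flag to choose between edge and center materials.
; An outline overlay material call is left unconnected, and the event graph holds only disabled default events.
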(fn `UserConstructionScript`
  (bind _cube (`self.Cube`))
  (`StaticMeshComponent.SetForceDisableNanite` _cube true)
  (`StaticMeshComponent.SetStaticMesh` _cube "/Game/_GENERATED/Dylan/Box_C23C4A53.Box_C23C4A53")
  (if (`self.EdgePeice`)
    (`PrimitiveComponent.SetMaterial` (`self.Cube`) 0 "/Game/Core/Materials/Color/MI_EdgePeice.MI_EdgePeice")
    (else
      (`PrimitiveComponent.SetMaterial` (`self.Cube`) 0 "/Game/Core/Materials/Color/MI_CenterPeice.MI_CenterPeice"))))