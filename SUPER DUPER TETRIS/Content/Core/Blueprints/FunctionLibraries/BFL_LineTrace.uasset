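; Blueprint function library with one helper, UpdateBeam, that fits a Niagara beam effect to a line trace.
; It traces on Visibility from a component's location along its negative up vector for a given distance.
; The component location feeds BeamBegin and the hit location feeds BeamEnd, with no check for a miss.
; Debug trace drawing and a print of the trace end remain active.
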(fn `UpdateBeam`
  (params (BeamParticalSystem :type "NiagaraComponent Object Reference") (StartingCube :type "StaticMeshComponent Object Reference") (EndPoint :type "Float (double-precision)" :default 1000.0))
  (bind _returnvalue (`SceneComponent.K2_GetComponentLocation` StartingCube))
  (bind _returnvalue_2 (+ _returnvalue (* (`SceneComponent.GetUpVector` StartingCube) (* EndPoint -1.0))))
  (`NiagaraComponent.SetVariableVec3` BeamParticalSystem "BeamBegin" _returnvalue)
  (`KismetSystemLibrary.PrintString` null (`KismetStringLibrary.Conv_VectorToString` _returnvalue_2))
  (bind _outhit (`KismetSystemLibrary.LineTraceSingle` :`Start` _returnvalue :`End` _returnvalue_2 :`TraceChannel` "TraceTypeQuery1" :`DrawDebugType` "ForDuration"))
  (`NiagaraComponent.SetVariableVec3` (`local.BeamParticalSystem`) "BeamEnd" (`.Location` (`GameplayStatics.BreakHitResult` _outhit))))