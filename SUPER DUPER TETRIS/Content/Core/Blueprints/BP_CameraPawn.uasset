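; BP_CameraPawn is a camera pawn that orbits and zooms on a spring arm.
; While left mouse is held, Tick applies mouse axes to arm rotation with clamped pitch; on release, it eases back to the BeginPlay rotation using RInterpTo.
; IsCameraMoved, despite its name, returns true when the arm is at that default, stopping the return.
; The mouse wheel adjusts arm length without limits.
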(event `self.ReceiveBeginPlay`
  ;[1 1 1] Begin Play
  (set `self.DefaultRotation` (`SceneComponent.RelativeRotation` (`self.SpringArm`))))

(event `self.ReceiveTick`
  (params (DeltaSeconds :type "Float (single-precision)"))
  (bind _returnvalue (`KismetMathLibrary.RInterpTo` (`SceneComponent.RelativeRotation` (`self.SpringArm`)) (`self.DefaultRotation`) DeltaSeconds 2.0))
  ;[1 1 1] Move Camera Spring Arm
  (if (`self.IsMouseButtonDown`)
    (`SceneComponent.K2_SetRelativeRotation` (`self.SpringArm`) (`KismetMathLibrary.MakeRotator` (.roll (`SceneComponent.RelativeRotation` (`self.SpringArm`))) (`KismetMathLibrary.FClamp` (+ (.pitch (`SceneComponent.RelativeRotation` (`self.SpringArm`))) (* (stale `InputAxisKey|MouseY` AxisValue) (`self.OrbitSensitivity`))) -80.0 10.0) (+ (.yaw (`SceneComponent.RelativeRotation` (`self.SpringArm`))) (* (stale `InputAxisKey|MouseX` AxisValue) (`self.OrbitSensitivity`)))) false false)
    (else
      ;;[1 1 1] Return to default
      (if (not (`self.IsCameraMoved`))
        (`SceneComponent.K2_SetRelativeRotation` (`self.SpringArm`) _returnvalue false false)
        (`KismetSystemLibrary.PrintString` (`KismetStringLibrary.Conv_RotatorToString` _returnvalue) false)))))

(event `Key|LeftMouseButton`
  (params (Key :type "Key Structure"))
  ;[1 1 1] LMB Input
  (:`Pressed`
    (bind _output_get (set `self.IsMouseButtonDown` true)))
  (:`Released`
    (bind _output_get_2 (set `self.IsMouseButtonDown` false))))

(event `InputAxisKey|MouseY`
  (params (AxisValue :type "Float (single-precision)"))
  ;[1 1 1] Move Camera Spring Arm
)

(event `InputAxisKey|MouseX`
  (params (AxisValue :type "Float (single-precision)"))
  ;[1 1 1] Move Camera Spring Arm
)

(event `InputAxisKey|MouseWheelAxis`
  (params (AxisValue :type "Float (single-precision)"))
  (bind _springarm (`self.SpringArm`))
  ;[1 1 1] Zoom
  (set `SpringArmComponent.TargetArmLength` (- (`SpringArmComponent.TargetArmLength` _springarm) (* AxisValue (`self.ZoomSensitivity`))) _springarm))

(fn `IsCameraMoved`
  (returns (ReturnValue :type Boolean))
  (return (== (`KismetMathLibrary.MakeTransform` (0.0 0.0 0.0) (`self.DefaultRotation`)) (`KismetMathLibrary.MakeTransform` (0.0 0.0 0.0) (`SceneComponent.RelativeRotation` (`self.SpringArm`))))))

(fn `UserConstructionScript`)