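; L-shaped Tetris piece Blueprint that projects a beam from one of its cubes to the surface below it.
; UpdateBeam runs on construction and every Tick, line-tracing along Cube2's negative up vector and feeding the start and hit location into the Beam's vector variables.
; The function ignores the cube and endpoint its callers pass, does not check for a hit, and leaves debug printing and trace drawing active.
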(event `self.ReceiveTick`
  (params (DeltaSeconds :type "Float (single-precision)"))
  (`/Game/Core/Blueprints/FunctionLibraries/BFL_LineTrace.UpdateBeam` (`self.Beam`) (`self.Cube3`)))

(fn `UpdateBeam`
  (bind _cube2 (`self.Cube2`))
  (bind _returnvalue (`SceneComponent.K2_GetComponentLocation` _cube2))
  (bind _returnvalue_2 (+ _returnvalue (* (`SceneComponent.GetUpVector` _cube2) -2000.0)))
  (`NiagaraComponent.SetVariableVec3` (`self.Beam`) "BeamBegin" _returnvalue)
  (`KismetSystemLibrary.PrintString` (`KismetStringLibrary.Conv_VectorToString` _returnvalue_2))
  (bind _outhit (`KismetSystemLibrary.LineTraceSingle` :`Start` _returnvalue :`End` _returnvalue_2 :`TraceChannel` "TraceTypeQuery1" :`DrawDebugType` "ForDuration"))
  (`NiagaraComponent.SetVariableVec3` (`self.Beam`) "BeamEnd" (`.Location` (`GameplayStatics.BreakHitResult` _outhit))))

(fn `UserConstructionScript`
  (`parent.UserConstructionScript`)
  (`/Game/Core/Blueprints/FunctionLibraries/BFL_LineTrace.UpdateBeam` (`self.Beam`) (`self.Cube_0`)))