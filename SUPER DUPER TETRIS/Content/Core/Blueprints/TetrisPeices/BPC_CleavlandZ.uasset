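; BPC_CleavlandZ is the Blueprint for the Cleveland Z Tetris piece, with a vertical beam that extends below it.
; SetBeam feeds the Beam effect a start at Cube1's world location and an end a fixed distance straight down in world Z, with no trace.
; It runs after the parent construction script and again every Tick, so the beam follows the piece and stays vertical when it rotates.
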(event `self.ReceiveTick`
  (params (DeltaSeconds :type "Float (single-precision)"))
  (`self.SetBeam`))

(fn `SetBeam`
  (`NiagaraComponent.SetVariableVec3` (`self.Beam`) "BeamBegin" (`SceneComponent.K2_GetComponentLocation` (`self.Cube_1`)))
  (`NiagaraComponent.SetVariableVec3` (`self.Beam`) "BeamEnd" (+ (`SceneComponent.K2_GetComponentLocation` (`self.Cube_1`)) (0.0 0.0 -1000.0))))

(fn `UserConstructionScript`
  (`parent.UserConstructionScript`)
  (`self.SetBeam`))