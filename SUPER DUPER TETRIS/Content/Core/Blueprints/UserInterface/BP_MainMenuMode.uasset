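; Main menu mode Blueprint that spawns random Tetris pieces at the level's TargetPoints, apparently as menu decoration.
; BeginPlay gathers and shuffles the TargetPoints, then starts a one-second timer whose looping follows IsLooping.
; Each tick of the timer advances Index and spawns a random piece class at that point.
; At the last index it only sets IsLooping false, without clearing the timer.
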(event `self.ReceiveBeginPlay`
  (bind _outactors (`GameplayStatics.GetAllActorsOfClass` "/Script/Engine.TargetPoint"))
  (bind _output_get (set `self.TargetPoints` _outactors))
  (bind _output_get_2 (set `self.TargetPointsShuffled` _output_get))
  (`KismetArrayLibrary.Array_Shuffle` _output_get_2)
  (`KismetSystemLibrary.K2_SetTimerDelegate` (delegate `Spawn Peice`) 1.0 (`self.IsLooping`)))

(event `Spawn Peice`
  (`self.SpawnPeiceRandom` (`self.TargetPointsShuffled`)))

(fn `SpawnPeiceRandom`
  (params (ArrayIn :type "Array of TargetPoint Object Reference"))
  (bind _tetrrispecies (`self.TetrrisPecies`))
  (if (== (`self.Index`) (`KismetArrayLibrary.Array_LastIndex` (`local.ArrayIn`)))
    (set `self.IsLooping` false)
    (else
      (`/Engine/EditorBlueprintResources/StandardMacros.IncrementInt` (`self.Index`)
        (:`  `
          (`|SpawnActorFromClass` (`|GetArrayItem` _tetrrispecies (`KismetMathLibrary.RandomIntegerInRange` 0 (`KismetArrayLibrary.Array_LastIndex` _tetrrispecies))) (`self.GetTransform` (`|GetArrayItem` (`local.ArrayIn`) (`self.Index`))) "AdjustIfPossibleButAlwaysSpawn" "MultiplyWithRoot" null null)
          (return))))))

(fn `UserConstructionScript`)