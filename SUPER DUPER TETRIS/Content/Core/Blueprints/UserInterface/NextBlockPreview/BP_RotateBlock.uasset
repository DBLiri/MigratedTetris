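; BP_RotateBlock is an actor that renders a spinning 3D preview of a block piece, filed under the next-block preview UI.
; Tick slowly yaws the scene root and restricts the SceneCaptureComponent2D to show only the piece's static mesh, isolating it from the world.
; SetModel takes a piece struct and applies its model and first-slot material to that mesh.
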(event `self.ReceiveBeginPlay`)

(event `self.ReceiveTick`
  (params (DeltaSeconds :type "Float (single-precision)"))
  (`SceneComponent.K2_AddLocalRotation` (`self.Scene`) (`KismetMathLibrary.MakeRotator` 0.0 0.0 (* DeltaSeconds 15.0)) false false)
  (`SceneCaptureComponent.ShowOnlyComponent` (`self.SceneCaptureComponent2D`) (`self.StaticMesh`)))

(fn `SetModel`
  (params (CurrentPeiceStruct :type "/Game/Core/Blueprints/TetrisPeices/S_FakePeices Structure"))
  (bind (_piecebp _name _image _piecemodel _material) (break `/Game/Core/Blueprints/TetrisPeices/S_FakePeices` CurrentPeiceStruct))
  (`SceneComponent.K2_SetRelativeLocationAndRotation` :`self` (`self.Scene`) :`NewLocation` (`SceneComponent.RelativeLocation` (`self.Scene`)))
  (`StaticMeshComponent.SetStaticMesh` (`self.StaticMesh`) _piecemodel)
  (`PrimitiveComponent.SetMaterial` (`self.StaticMesh`) 0 _material))

(fn `UserConstructionScript`
  (`PrimitiveComponent.SetMaterial` (`self.StaticMesh`) 0 null))